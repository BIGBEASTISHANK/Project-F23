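; BP_GameMode is the game mode that sets up the in-game player HUD and keeps the player's health within range.
; BeginPlay creates the WB_PlayerInGameUI widget, which holds the health bar, and adds it to the viewport.
; Every Tick casts player character 0 to BP_Player, clamps its Health between zero and MaxHealth, and prints the value as debug text.
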(event `self.ReceiveBeginPlay`
  ;[0 0 0] Adding Health Bar to viewport
  (bind _returnvalue (`|CreateWidget` "/Game/Core/Player/UI/WB_PlayerInGameUI.WB_PlayerInGameUI_C"))
  (`UserWidget.AddToViewport` _returnvalue 0))

(event `self.ReceiveTick`
  (params (DeltaSeconds :type "Float (single-precision)"))
  ;[0 0 0] Getting Player Refrence
  (bind _asbp_player (cast `/Game/Core/Player/BP_Player` (`GameplayStatics.GetPlayerCharacter` 0)))
  (bind _output_get (set `self.Player Ref` _asbp_player))
  ;[0 0 0] Health should not exceed Max Health
  (if (> (`/Game/Core/Player/BP_Player.Health` _output_get) (`/Game/Core/Player/BP_Player.Max Health` _output_get))
    (set `/Game/Core/Player/BP_Player.Health` (`/Game/Core/Player/BP_Player.Max Health` _output_get) _output_get))
  ;[0 0 0] Health should not go below 0
  (if (< (`/Game/Core/Player/BP_Player.Health` _output_get) 0.0)
    (set `/Game/Core/Player/BP_Player.Health` 0.0 _output_get))
  (`KismetSystemLibrary.PrintString` (`KismetStringLibrary.Conv_DoubleToString` (`/Game/Core/Player/BP_Player.Health` (`self.Player Ref`))) true true (struct :`G` 0.66 :`B` 1.0 :`A` 1.0) 2.0 "Health"))

(fn `UserConstructionScript`)